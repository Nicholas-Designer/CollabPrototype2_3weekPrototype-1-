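; Base pickup actor for collectables, counted by type as coins, scrap or blueprints.
; On sphere overlap it offers its amount and collectable type to the other actor through an interface message.
; If that returns true, it notifies the game mode through the interface message matching the type, with blueprints as the fallback, then destroys itself.
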(event `self.Sphere1.OnComponentBeginOverlap`
  (params (OverlappedComponent :type "PrimitiveComponent Object Reference") (OtherActor :type "Actor Object Reference") (OtherComp :type "PrimitiveComponent Object Reference") (OtherBodyIndex :type Integer) (bFromSweep :type Boolean) (SweepResult :type "HitResult Structure (by ref)"))
  (bind _returnvalue (`GameplayStatics.GetGameMode`))
  (bind _collectableinventory (`self.CollectableInventory`))
  (bind _shoulddestroy (message `/Game/Tech/THOMPSON_Joshua/New/BPI_Character.I_AddCollectables` OtherActor (`self.AddingInt`) (`self.CollectableInventory`)))
  (if _shoulddestroy
    (if (`|EnumEquality` _collectableinventory "NewEnumerator0")
      ;[1 1 1] Interface for the active task
      (message `/Game/Tech/THOMPSON_Joshua/ObjectiveManager/BPI_GameMode.I_UpdateCollectedCoins` _returnvalue)
      (elif (`|EnumEquality` _collectableinventory "NewEnumerator5")
        (message `/Game/Tech/THOMPSON_Joshua/ObjectiveManager/BPI_GameMode.I_UpdateCollectedScrap` _returnvalue)
        (else
          (message `/Game/Tech/THOMPSON_Joshua/ObjectiveManager/BPI_GameMode.I_UpdateCollectedBlueprints` _returnvalue))))
    (`self.K2_DestroyActor`)))

(fn `UserConstructionScript`)