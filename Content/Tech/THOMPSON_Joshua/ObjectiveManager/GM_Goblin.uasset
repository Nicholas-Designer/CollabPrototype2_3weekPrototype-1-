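; Goblin game mode that acts as a prototype objective manager for a main task and coin or scrap sub-tasks.
; BeginPlay creates both objective widgets and randomly activates a blueprint, chest or useless-item task, rolling its displayed text separately.
; Interface events count progress for active tasks, show sub-task text and enable sub-tasks while ActiveSubTask, never set here, is false.
; Completion only prints for coins and chests; other branches are empty.
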(event `self.ReceiveBeginPlay`
  (bind _returnvalue (`KismetMathLibrary.RandomInteger` 3))
  (bind _returnvalue_2 (`|CreateWidget` "/Game/Tech/THOMPSON_Joshua/ObjectiveManager/BPW_CurrentObjective.BPW_CurrentObjective_C"))
  (bind _output_get (set `self.Current Objective` _returnvalue_2))
  (`UserWidget.AddToViewport` _output_get 0)
  (message `/Game/Tech/THOMPSON_Joshua/ObjectiveManager/BPI_ObjectiveManagerWidgets.I_ChangeTextColour` _output_get (struct :`R` 1.0 :`G` 1.0 :`B` 1.0 :`A` 1.0))
  (message `/Game/Tech/THOMPSON_Joshua/ObjectiveManager/BPI_ObjectiveManagerWidgets.I_ChangeText` _output_get (`|GetArrayItem` (`self.Tasks List`)))
  (bind _returnvalue_3 (`|CreateWidget` "/Game/Tech/THOMPSON_Joshua/ObjectiveManager/BPW_SubObjective.BPW_SubObjective_C"))
  (bind _output_get_2 (set `self.Sub Objective` _returnvalue_3))
  (`UserWidget.AddToViewport` _output_get_2 0)
  (`Widget.SetVisibility` _output_get_2 "Hidden")
  (message `/Game/Tech/THOMPSON_Joshua/ObjectiveManager/BPI_ObjectiveManagerWidgets.I_ChangeTextColour` _output_get_2 (struct :`R` 0.869792 :`G` 0.869792 :`B` 0.869792 :`A` 1.0))
  (switch `int` _returnvalue
    (:`0`
      (set `self.Blueprint Task Active` true))
    (:`1`
      (set `self.Chest Task Active` true))
    (:`2`
      (set `self.Useless Item Task Active` true)))
  (message `/Game/Tech/THOMPSON_Joshua/ObjectiveManager/BPI_ObjectiveManagerWidgets.I_ChangeText` (`self.Current Objective`) (`|GetArrayItem` (`self.Tasks List`) _returnvalue)))

(event `/Game/Tech/THOMPSON_Joshua/ObjectiveManager/BPI_GameMode.I_BoughtUselessItem`
  (if (`self.Useless Item Task Active`)
    (bind _output_get (set `self.BoughtUselessItem` true))
    (if (== _output_get true)
      _)))

(event `/Game/Tech/THOMPSON_Joshua/ObjectiveManager/BPI_GameMode.I_UpdateCollectedScrap`
  (if (`self.Scrap Task Active`)
    (bind _output_get (set `self.CollectedScrap` (+ (`self.CollectedScrap`) 1)))
    (if (== _output_get 20)
      _)))

(event `/Game/Tech/THOMPSON_Joshua/ObjectiveManager/BPI_GameMode.I_UpdateCollectedCoins`
  (if (`self.Coin Task Active`)
    (bind _output_get (set `self.CollectedCoins` (+ (`self.CollectedCoins`) 1)))
    (`KismetSystemLibrary.PrintString` "Collected Coins")
    (if (== _output_get 20)
      (`KismetSystemLibrary.PrintString` "Collected 20 Coins"))))

(event `/Game/Tech/THOMPSON_Joshua/ObjectiveManager/BPI_GameMode.I_UpdateCollectedBlueprints`
  (if (`self.Blueprint Task Active`)
    (bind _output_get (set `self.CollectedBlueprints` (+ (`self.CollectedBlueprints`) 1)))
    (if (== _output_get 10)
      _)))

(event `/Game/Tech/THOMPSON_Joshua/ObjectiveManager/BPI_GameMode.I_UpdateOpenedChests`
  (if (`self.Chest Task Active`)
    (bind _output_get (set `self.OpenedChests` (+ (`self.OpenedChests`) 1)))
    (if (== _output_get 3)
      (`KismetSystemLibrary.PrintString` "Completed Task")
      (else
        (`KismetSystemLibrary.PrintString` "Opened Chest")))))

(event `/Game/Tech/THOMPSON_Joshua/ObjectiveManager/BPI_GameMode.I_UpdateSubTask`
  (params (Task :type Integer))
  (message `/Game/Tech/THOMPSON_Joshua/ObjectiveManager/BPI_ObjectiveManagerWidgets.I_ChangeText` (`self.Sub Objective`) (`|GetArrayItem` (`self.Sub Tasks`) (- Task 1)))
  (`Widget.SetVisibility` (`self.Sub Objective`) "Visible"))

(fn `I_SetCoinsActiveSubTask`
  (returns (`Sub Task Active ` :type Boolean))
  (if (== (`self.ActiveSubTask`) false)
    (set `self.Coin Task Active` true)
    (return false)
    (else
      (return true))))

(fn `I_SetScrapActiveSubTask`
  (returns (`Sub Task Active` :type Boolean))
  (if (== (`self.ActiveSubTask`) false)
    (set `self.Scrap Task Active` true)
    (return false)
    (else
      (return true))))

(fn `UserConstructionScript`)