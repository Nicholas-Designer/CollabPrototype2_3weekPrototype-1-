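; Objective manager that shows the player's current main objective and an optional sub-objective through on-screen widgets.
; Interface events report scrap and coin milestones, briefly flashing the matching text green, then advancing the main task or hiding the sub-objective.
; Reaching the second scrap milestone shows a finish widget, pauses the game and switches to UI-only input.
; Other interface calls set sub-quest text, visibility and active flags, or query those flags; the spotted event does nothing.
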(event `self.ReceiveBeginPlay`
  (bind _returnvalue (`|CreateWidget` "/Game/Tech/THOMPSON_Joshua/ObjectiveManager/BPW_CurrentObjective.BPW_CurrentObjective_C"))
  (bind _output_get (set `self.CurrentObjectiveUI` _returnvalue))
  (`UserWidget.AddToViewport` _output_get 0)
  (message `/Game/Tech/THOMPSON_Joshua/ObjectiveManager/BPI_ObjectiveManagerWidgets.I_ChangeTextColour` _output_get (struct :`R` 1.0 :`G` 1.0 :`B` 1.0 :`A` 1.0))
  (message `/Game/Tech/THOMPSON_Joshua/ObjectiveManager/BPI_ObjectiveManagerWidgets.I_ChangeText` _output_get (`|GetArrayItem` (`self.Task List`)))
  (bind _returnvalue_2 (`|CreateWidget` "/Game/Tech/THOMPSON_Joshua/ObjectiveManager/BPW_SubObjective.BPW_SubObjective_C"))
  (bind _output_get_2 (set `self.SubObjectiveUI` _returnvalue_2))
  (`UserWidget.AddToViewport` _output_get_2 0)
  (`Widget.SetVisibility` _output_get_2 "Hidden")
  (message `/Game/Tech/THOMPSON_Joshua/ObjectiveManager/BPI_ObjectiveManagerWidgets.I_ChangeTextColour` _output_get_2 (struct :`R` 0.869792 :`G` 0.869792 :`B` 0.869792 :`A` 1.0)))

(event `/Game/Tech/THOMPSON_Joshua/ObjectiveManager/BPI_ObjectiveManager.I_ScrapCollected10`
  (if (not (`self.Collected_10_Scrap`))
    (`self.CompletedColourChange` (`self.CurrentObjectiveUI`))
    (`KismetSystemLibrary.Delay` (`self.DelayTime`))
    (message `/Game/Tech/THOMPSON_Joshua/ObjectiveManager/BPI_ObjectiveManagerWidgets.I_ChangeText` (`self.CurrentObjectiveUI`) (`|GetArrayItem` (`self.Task List`) 1))
    (set `self.Collected_10_Scrap` true)))

(event `/Game/Tech/THOMPSON_Joshua/ObjectiveManager/BPI_ObjectiveManager.I_ScrapCollected20`
  (if (not (`self.Collected_20_Scrap`))
    (`self.CompletedColourChange` (`self.CurrentObjectiveUI`))
    (`KismetSystemLibrary.Delay` (`self.DelayTime`))
    (bind _returnvalue (`|CreateWidget` "/Game/Tech/THOMPSON_Joshua/ObjectiveManager/BPW_Finished.BPW_Finished_C"))
    (bind _output_get (set `self.FinishUI` _returnvalue))
    (`UserWidget.AddToViewport` _output_get 0)
    (`GameplayStatics.SetGamePaused` true)
    (`WidgetBlueprintLibrary.SetInputMode_UIOnlyEx` (`GameplayStatics.GetPlayerController` 0) (`self.FinishUI`))))

(event `/Game/Tech/THOMPSON_Joshua/ObjectiveManager/BPI_ObjectiveManager.I_Spotted`
  (if (`self.Spotted`)
    _))

(event `/Game/Tech/THOMPSON_Joshua/ObjectiveManager/BPI_ObjectiveManager.I_CollectedCoins10`
  (bind _subobjectiveui (`self.SubObjectiveUI`))
  (if (not (`self.Collected_10_Coins`))
    (`self.CompletedColourChange` _subobjectiveui)
    (`KismetSystemLibrary.Delay` (`self.DelayTime`))
    (`Widget.SetVisibility` _subobjectiveui "Hidden")
    (`KismetArrayLibrary.Array_Set` (`self.SubActiveArray`))
    (set `self.Collected_10_Coins` true)))

(event `CompletedColourChange`
  (params (`UI Ref` :type "Object Object Reference"))
  (message `/Game/Tech/THOMPSON_Joshua/ObjectiveManager/BPI_ObjectiveManagerWidgets.I_ChangeTextColour` `UI Ref` (struct :`G` 0.869792 :`B` 0.009819 :`A` 1.0))
  (`KismetSystemLibrary.Delay` (`self.DelayTime`))
  (message `/Game/Tech/THOMPSON_Joshua/ObjectiveManager/BPI_ObjectiveManagerWidgets.I_ChangeTextColour` `UI Ref` (struct :`R` 1.0 :`G` 1.0 :`B` 1.0 :`A` 1.0)))

(event `/Game/Tech/THOMPSON_Joshua/ObjectiveManager/BPI_ObjectiveManager.I_SetSubQuest`
  (params (SubQuest :type Integer))
  (`KismetArrayLibrary.Array_Set` (`self.SubActiveArray`) SubQuest true)
  (message `/Game/Tech/THOMPSON_Joshua/ObjectiveManager/BPI_ObjectiveManagerWidgets.I_ChangeText` (`self.SubObjectiveUI`) (`|GetArrayItem` (`self.SubTextArray`) SubQuest)))

(event `/Game/Tech/THOMPSON_Joshua/ObjectiveManager/BPI_ObjectiveManager.I_HideUI`
  (params (`UI Visibilty` :type "ESlateVisibility Enum" :default "Visible") (CurrnetSubTask :type Integer))
  (`Widget.SetVisibility` (`self.SubObjectiveUI`) `UI Visibilty`)
  (`KismetArrayLibrary.Array_Set` (`self.SubActiveArray`) CurrnetSubTask true))

(fn `I_GetSubArray`
  (params (Elm :type Integer))
  (returns (ActiveState :type Boolean))
  (return (`|GetArrayItem` (`self.SubActiveArray`) Elm)))

(fn `UserConstructionScript`)