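; Player controller for a third-person game that forwards player input to the controlled pawn.
; Movement, look, jump, interact, item picker and item use inputs become interface messages on the pawn, keeping the controller free of pawn-specific logic.
; An IStoreOpen event sets an Open flag that blocks item picking and use while the store is open.
; Jump press and release both send the same pressed message.
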(event `InputAction|ItemPickerRight`
  (params (Key :type "Key Structure"))
  ;[1 1 1 1 106] T017789k
  ;;[1 1 1] For the item picker on the UI
  (:`Pressed`
    (if (not (`self.Open`))
      (message `/Game/Tech/THOMPSON_Joshua/My3rdPerson/BPI_ButtonPresses.I_ItemPick` (`self.K2_GetPawn`) true))))

(event `InputAction|ItemPickerLeft`
  (params (Key :type "Key Structure"))
  ;[1 1 1 1 106] T017789k
  ;;[1 1 1] For the item picker on the UI
  (:`Pressed`
    (if (not (`self.Open`))
      (message `/Game/Tech/THOMPSON_Joshua/My3rdPerson/BPI_ButtonPresses.I_ItemPick` (`self.K2_GetPawn`) false))))

(event `InputAction|UseItems`
  (params (Key :type "Key Structure"))
  (bind _returnvalue (`self.K2_GetPawn`))
  (bind _returnvalue_2 (not (`self.Open`)))
  ;[1 1 1 1 106] T017789k
  ;;[1 1 1] Using Item from Inventory
  (:`Pressed`
    (if _returnvalue_2
      (message `/Game/Tech/THOMPSON_Joshua/My3rdPerson/BPI_ButtonPresses.I_UseItemPressed` _returnvalue)))
  (:`Released`
    (if _returnvalue_2
      (message `/Game/Tech/THOMPSON_Joshua/My3rdPerson/BPI_ButtonPresses.I_UseItemReleased` _returnvalue))))

(event `InputAction|Interact`
  (params (Key :type "Key Structure"))
  (bind _returnvalue (`self.K2_GetPawn`))
  ;[1 1 1 1 106] T017789k
  ;;[1 1 1] Interaction Button Press
  (:`Pressed`
    (message `/Game/Tech/THOMPSON_Joshua/My3rdPerson/BPI_ButtonPresses.I_InteractButtonPressed` _returnvalue))
  (:`Released`
    (message `/Game/Tech/THOMPSON_Joshua/My3rdPerson/BPI_ButtonPresses.I_InteractButtonReleased` _returnvalue)))

(event `InputAxis|MoveForward`
  (params (AxisValue :type "Float (single-precision)"))
  ;[1 1 1 1 106] T017789k
  ;;[1 1 1] Basic Movement
  (message `/Game/Tech/THOMPSON_Joshua/My3rdPerson/BPI_ButtonPresses.I_InputAxisForward` (`self.K2_GetPawn`) AxisValue))

(event `InputAxis|MoveRight`
  (params (AxisValue :type "Float (single-precision)"))
  ;[1 1 1 1 106] T017789k
  ;;[1 1 1] Basic Movement
  (message `/Game/Tech/THOMPSON_Joshua/My3rdPerson/BPI_ButtonPresses.I_InputAxisRight` (`self.K2_GetPawn`) AxisValue))

(event `InputAxis|Turn`
  (params (AxisValue :type "Float (single-precision)"))
  ;[1 1 1 1 106] T017789k
  ;;[1 1 1] Basic Movement
  (message `/Game/Tech/THOMPSON_Joshua/My3rdPerson/BPI_ButtonPresses.I_InputAxisTurn` (`self.K2_GetPawn`) AxisValue))

(event `InputAxis|LookUp`
  (params (AxisValue :type "Float (single-precision)"))
  ;[1 1 1 1 106] T017789k
  ;;[1 1 1] Basic Movement
  (message `/Game/Tech/THOMPSON_Joshua/My3rdPerson/BPI_ButtonPresses.I_InputAxisLookUp` (`self.K2_GetPawn`) AxisValue))

(event `InputAction|Jump`
  (params (Key :type "Key Structure"))
  (bind _returnvalue (`self.K2_GetPawn`))
  ;[1 1 1 1 106] T017789k
  ;;[1 1 1] Basic Movement
  (:`Pressed`
    (message `/Game/Tech/THOMPSON_Joshua/My3rdPerson/BPI_ButtonPresses.I_JumpPressed` _returnvalue))
  (:`Released`
    (message `/Game/Tech/THOMPSON_Joshua/My3rdPerson/BPI_ButtonPresses.I_JumpPressed` _returnvalue)))

(event `/Game/Tech/THOMPSON_Joshua/My3rdPerson/BPI_PlayerController.I_StoreOpen`
  (params (Open :type Boolean))
  ;[1 1 1 1 106] T017789k
  ;;[1 1 1] Used so you dont use items when the store is open
  (set `self.Open` Open))

(fn `UserConstructionScript`)