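; BP_GrappleHook is a grapple hook projectile actor that flies in a straight line to a Target actor and stops there.
; BeginPlay caches start and end locations and sets the ProjectileMovement velocity along that direction at Speed.
; Tick compares squared distances from the start to catch overshoot against the Target's current location, then snaps the hook to the cached end point and zeroes velocity.
; DistanceToTarget exposes the remaining distance.
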(event `self.ReceiveBeginPlay`
  (set `self.StartLocation` (`self.K2_GetActorLocation`))
  (set `self.EndLocation` (`self.K2_GetActorLocation` (`self.Target`)))
  (set `self.Direction` (`KismetMathLibrary.Normal` (- (`self.EndLocation`) (`self.StartLocation`))))
  (set `MovementComponent.Velocity` (* (`self.Direction`) (`self.Speed`)) (`self.ProjectileMovement`)))

(event `self.ReceiveTick`
  (params (DeltaSeconds :type "Float (single-precision)"))
  (if (>= (`KismetMathLibrary.Vector_DistanceSquared` (`self.K2_GetActorLocation`) (`self.StartLocation`)) (`KismetMathLibrary.Vector_DistanceSquared` (`self.K2_GetActorLocation` (`self.Target`)) (`self.StartLocation`)))
    (`self.K2_SetActorLocation` (+ (`self.StartLocation`) (* (`self.Direction`) (`KismetMathLibrary.Vector_Distance` (`self.StartLocation`) (`self.EndLocation`)))))
    (set `MovementComponent.Velocity` (0.0 0.0 0.0) (`self.ProjectileMovement`))))

(fn `DistanceToTarget`
  (returns (ReturnValue :type "Float (double-precision)"))
  (return (`KismetMathLibrary.Vector_Distance` (`self.EndLocation`) (`self.K2_GetActorLocation`))))

(fn `UserConstructionScript`)